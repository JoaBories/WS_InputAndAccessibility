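; Obstacle actor that kills the player on sphere overlap, or destroys itself and adds a score point on hitting a Wall-tagged actor.
; A kill removes the obstacle spawner, ragdolls the character and shows the death widget, adding blood and sound when gore is enabled.
; BeginPlay caches the character and game instance, whose gore and VFX settings drive the mesh choice and the Niagara components' pause and rendering states.
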(event OnComponentBeginOverlap(Sphere)
  (params (OverlappedComponent :type Primitive%20Component%20Object%20Reference) (OtherActor :type Actor%20Object%20Reference) (OtherComp :type Primitive%20Component%20Object%20Reference) (OtherBodyIndex :type Integer) (bFromSweep :type Boolean) (SweepResult :type Hit%20Result%20Structure%20%28by%20ref%29))
  (if (== OtherActor (Game|GetPlayerCharacter 0))
    (CallFunction|KillPlayer)
    (elif (Actor|ActorHasTag OtherActor "Wall")
      (Actor|DestroyActor)
      (Math|Integer|IncrementInt (Variables|/Game/Paul/BP/BP_Chara.BP_Chara_C|GetScore (Variables|Default|GetChara))))))

(event Custom|KillPlayer
  (bind _returnvalue (Actor|GetActorOfClass "/Game/Joa/BP_ObstacleSpawner.BP_ObstacleSpawner_C"))
  (Utilities|IsValid _returnvalue
    (:Is%20Valid
      (Actor|DestroyActor _returnvalue)
      (Default|DieRagdoll (Variables|Default|GetChara))
      (if (Variables|/Game/Joa/GI_Custom.GI_Custom_C|GetGore_Activated (Variables|Default|GetGameInstance))
        (Niagara|SpawnSystematLocation "/Game/Paul/VFX/NS_Blood.NS_Blood" (Transformation|GetActorLocation (Variables|Default|GetChara)))
        (Audio|PlaySound2D "/Game/Paul/SoundFX/SC_DeadGore.SC_DeadGore" 1.0 1.0 0.0 0 0))
      (bind _returnvalue_2 (UserInterface|CreateWidget "/Game/UI/WBP_Dead.WBP_Dead_C"))
      (UserInterface|Viewport|AddtoViewport _returnvalue_2 0))))

(event EventActivateGore
  (params (Activate :type Boolean))
  ;[0.15 0.15 0.15 0.5] Deactivate Interface
  (Components|StaticMesh|SetStaticMesh (Variables|Default|GetStaticMesh) (select Activate "/Game/Paul/Mesh/StaticMesh.StaticMesh" "/Game/Template/LevelPrototyping/Meshes/SM_ChamferCube.SM_ChamferCube")))

(event EventBeginPlay
  ;[0.15 0.15 0.15 0.5] Deactivate Interface
  ;;[0.15 0.15 0.15 0.5] Begin Play
  (bind _asgi_custom (Utilities|Casting|CastToGI_Custom (Game|GetGameInstance)))
  (bind _output_get (Variables|Default|SetGameInstance _asgi_custom))
  (CallFunction|ActivateGore (Variables|/Game/Joa/GI_Custom.GI_Custom_C|GetGore_Activated _output_get))
  (CallFunction|ActiveVFX (Variables|/Game/Joa/GI_Custom.GI_Custom_C|GetVFX_Activated _output_get))
  (bind _asbp_chara (Utilities|Casting|CastToBP_Chara (Game|GetPlayerCharacter 0)))
  (Variables|Default|SetChara _asbp_chara))

(event EventActiveVFX
  (params (Activate :type Boolean))
  (bind _returnvalue (not Activate))
  ;[0.15 0.15 0.15 0.5] Deactivate Interface
  (for _array_element (Utilities|Array|MakeArray (Variables|Default|GetNiagara) (Variables|Default|GetNiagara1))
    (Class|NiagaraComponent|SetPaused _array_element _returnvalue)
    (Class|NiagaraComponent|SetRenderingEnabled _array_element _returnvalue)))

(fn ConstructionScript)