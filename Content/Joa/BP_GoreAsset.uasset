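; Blueprint for a prop that shows either a gore or a non-gore static mesh, following the game's gore setting.
; The construction script assigns GoreMesh by default.
; On BeginPlay it casts the game instance to GI_Custom, stores it and passes its GoreActivated flag to ActivateGore.
; The ActivateGore event sets the mesh component to GoreMesh or NotGoreMesh from its Activate input.
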(event EventActivateGore
  (params (Activate :type Boolean))
  (Components|StaticMesh|SetStaticMesh (Variables|Default|GetStaticMesh) (select Activate (Variables|Default|GetGoreMesh) (Variables|Default|GetNotGoreMesh))))

(event EventBeginPlay
  ;[0.15 0.15 0.15 0.5] Begin Play
  (bind _asgi_custom (Utilities|Casting|CastToGI_Custom (Game|GetGameInstance)))
  (bind _output_get (Variables|Default|SetGame%20Instance _asgi_custom))
  (CallFunction|ActivateGore (Variables|/Game/Joa/GI_Custom.GI_Custom_C|GetGore_Activated _output_get)))

(fn ConstructionScript
  (Components|StaticMesh|SetStaticMesh (Variables|Default|GetStaticMesh) (Variables|Default|GetGoreMesh)))