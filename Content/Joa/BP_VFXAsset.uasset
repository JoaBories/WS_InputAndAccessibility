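; Placeable VFX actor that shows an assignable Niagara effect and reads a global VFX toggle from the game instance.
; The construction script assigns the VFX asset to the Niagara component.
; On BeginPlay it casts to GI_Custom, stores it and passes VFXActivated to ActiveVFX.
; ActiveVFX feeds the inverted flag to both pause and rendering, so an active state runs the simulation with rendering disabled.
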(event EventActiveVFX
  (params (Activate :type Boolean))
  (bind _returnvalue (not Activate))
  (bind _niagara (Variables|Default|GetNiagara))
  (Class|NiagaraComponent|SetPaused _niagara _returnvalue)
  (Class|NiagaraComponent|SetRenderingEnabled _niagara _returnvalue))

(event EventBeginPlay
  ;[0.15 0.15 0.15 0.5] Begin Play
  (bind _asgi_custom (Utilities|Casting|CastToGI_Custom (Game|GetGameInstance)))
  (bind _output_get (Variables|Default|SetGame%20Instance _asgi_custom))
  (CallFunction|ActiveVFX (Variables|/Game/Joa/GI_Custom.GI_Custom_C|GetVFX_Activated _output_get)))

(fn ConstructionScript
  (Class|NiagaraComponent|SetAsset (Variables|Default|GetNiagara) (Variables|Default|GetVFX) true))