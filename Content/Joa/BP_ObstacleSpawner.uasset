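; Obstacle spawner actor that periodically spawns BP_Obstacle actors from fixed spawn-point components.
; On BeginPlay, two looping timers drive it: one spawns a vertical row, the other, less frequent, spawns from a single horizontal spawner.
; Each row picks a random entry from Patterns, whose three flags decide which vertical spawners fire.
; A shared SpawnObstacle event selects the spawner by direction and index and copies its world location and rotation.
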(event Custom|SpawnObstacle
  (params (Horizontal :type Boolean) (Index :type Integer))
  (bind _vertspawner1 (Variables|Default|GetVertSpawner1))
  (bind _vertspawner2 (Variables|Default|GetVertSpawner2))
  (bind _vertspawner3 (Variables|Default|GetVertSpawner3))
  (bind _horizontalspawner1 (Variables|Default|GetHorizontalSpawner1))
  (bind _returnvalue (Utilities|Select :Index Index :Option%200 _vertspawner1 :Option%201 _vertspawner2 :Option%202 _vertspawner3))
  (bind _returnvalue_2 (Utilities|Select :Index Index :Option%200 _horizontalspawner1 :Option%201 0))
  (bind _returnvalue_3 (select Horizontal _returnvalue_2 _returnvalue))
  (Game|SpawnActorfromClass "/Game/Joa/BP_Obstacle.BP_Obstacle_C" (Math|Transform|MakeTransform (Transformation|GetWorldLocation _returnvalue_3) (Transformation|GetWorldRotation _returnvalue_3) "1.000000,1.000000,1.000000") "Undefined" "MultiplyWithRoot" 0 0))

(event Custom|SpawnRow
  (bind _patterns (Variables|Default|GetPatterns))
  (bind _output_get (Variables|Default|SetRandomPattern (Math|Random|RandomInteger (Utilities|Array|Length _patterns))))
  (if (.vert1 (Utilities|Array|Get(acopy) _patterns _output_get))
    (CallFunction|SpawnObstacle false))
  (if (.vert2 (Utilities|Array|Get(acopy) _patterns _output_get))
    (CallFunction|SpawnObstacle false 1))
  (if (.vert3 (Utilities|Array|Get(acopy) _patterns _output_get))
    (CallFunction|SpawnObstacle false 2)))

(event Custom|SpawnHorizontal
  (CallFunction|SpawnObstacle true))

(event EventBeginPlay
  (Utilities|Time|SetTimerbyEvent (delegate Custom|SpawnRow) 5.0 true)
  (Utilities|Time|SetTimerbyEvent (delegate Custom|SpawnHorizontal) 7.0 true false 0.5))

(fn ConstructionScript)